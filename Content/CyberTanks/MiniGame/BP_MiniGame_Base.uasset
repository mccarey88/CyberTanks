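; Base pawn for station-module minigames, opened to recharge energy, repair HP or fully restore a station.
; On possession it renders its scene capture into the controller's render target and shows it in a widget placed at the station's screen position.
; Success applies the restore chosen by the minigame reason and returns to the station module; Fail, also triggered by the exit input, damages the station and returns to the character.
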(event `self.ReceivePossessed`
  (params (NewController :type "Controller Object Reference"))
  ; Creating widget to view minigame
  (bind _aspc_mpgame (cast `/Game/CyberTanks/MultiPlayerSetup/PC_MPGame` NewController))
  (set `SceneCaptureComponent2D.TextureTarget` (`/Game/CyberTanks/MultiPlayerSetup/PC_MPGame.RenderTarget` _aspc_mpgame) (`self.SceneCaptureComponent2D`))
  (bind _returnvalue (`|CreateWidget` "/Game/CyberTanks/MiniGame/W_MiniGameView.W_MiniGameView_C" null (`/Game/CyberTanks/MultiPlayerSetup/PC_MPGame.RenderMaterial` _aspc_mpgame)))
  (set `self.GameView` _returnvalue)
  (`UserWidget.AddToViewport` _returnvalue 0)
  (bind _aspc_mpgame_2 (cast `/Game/CyberTanks/MultiPlayerSetup/PC_MPGame` (`self.GetController`)))
  (`Widget.SetRenderTransform` _returnvalue (make `WidgetTransform` (`WidgetLayoutLibrary.ProjectWorldLocationToWidgetPosition` (`GameplayStatics.GetPlayerController` 0) (`SceneComponent.K2_GetComponentLocation` (`/Game/CyberTanks/TankBase/Modules/BP_Module_Base.DefaultSceneRoot` (`/Game/CyberTanks/MultiPlayerSetup/PC_MPGame.StationModule` _aspc_mpgame_2)))))))

(event `EnhancedInput|/Game/ThirdPerson/Input/Actions/IA_Exit`
  (params (ActionValue :type Boolean) (ElapsedSeconds :type "Float (double-precision)") (TriggeredSeconds :type "Float (double-precision)") (InputAction :type "InputAction Object Reference" :default "/Game/ThirdPerson/Input/Actions/IA_Exit.IA_Exit"))
  (:`Triggered`
    (`self.Fail`)))

(event `Success`
  (`KismetSystemLibrary.PrintString` "MiniGame Success")
  (bind _aspc_mpgame (cast `/Game/CyberTanks/MultiPlayerSetup/PC_MPGame` (`self.GetController`)))
  (switch `/Game/CyberTanks/MiniGame/ENUM_WhyMiniGameStarted` (`self.ReasonForMiniGame`)
    (:`NewEnumerator0`
      _)
    (:`NewEnumerator1`
      (bind _ac_energon (`/Game/CyberTanks/TankBase/Modules/BP_Module_Base.AC_Energon` (`/Game/CyberTanks/MultiPlayerSetup/PC_MPGame.StationModule` _aspc_mpgame)))
      (`/Game/CyberTanks/EnergonComponent/AC_Energon.FullRestoreEnergy` _ac_energon true))
    (:`NewEnumerator2`
      (`/Game/CyberTanks/EnergonComponent/AC_Energon.FullRestoreHp` _ac_energon true))
    (:`NewEnumerator3`
      (`/Game/CyberTanks/EnergonComponent/AC_Energon.FullRestore` _ac_energon)))
  (`/Game/CyberTanks/MultiPlayerSetup/PC_MPGame.SwitchToStationModule` _aspc_mpgame (`/Game/CyberTanks/MultiPlayerSetup/PC_MPGame.StationModule` _aspc_mpgame))
  (`Widget.RemoveFromParent` (`self.GameView`))
  (`self.K2_DestroyActor`))

(event `Fail`
  (`KismetSystemLibrary.PrintString` "MiniGame Fail")
  (bind _aspc_mpgame (cast `/Game/CyberTanks/MultiPlayerSetup/PC_MPGame` (`self.GetController`)))
  (`/Game/CyberTanks/EnergonComponent/AC_Energon.Damage` (`/Game/CyberTanks/TankBase/Modules/BP_Module_Base.AC_Energon` (`/Game/CyberTanks/MultiPlayerSetup/PC_MPGame.StationModule` _aspc_mpgame)) 10.0 10.0)
  (`/Game/CyberTanks/MultiPlayerSetup/PC_MPGame.SwitchToCharacter` _aspc_mpgame)
  (`Widget.RemoveFromParent` (`self.GameView`))
  (`self.K2_DestroyActor`))

(fn `UserConstructionScript`)