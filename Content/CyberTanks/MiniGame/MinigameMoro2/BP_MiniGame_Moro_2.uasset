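; BP_MiniGame_Moro_2 is a tilt-platform ball minigame in which the player tips Platforma to steer the ball (Kula).
; IA_Move input is normalized, scaled by Sensivity and added to the platform's roll and pitch, which are then clamped to a limited tilt with yaw reset.
; Box calls Success when overlapped by a component tagged "K", while Box1 calls Fail when Kula enters it.
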(event `self.Box.OnComponentBeginOverlap`
  (params (OverlappedComponent :type "PrimitiveComponent Object Reference") (OtherActor :type "Actor Object Reference") (OtherComp :type "PrimitiveComponent Object Reference") (OtherBodyIndex :type Integer) (bFromSweep :type Boolean) (SweepResult :type "HitResult Structure (by ref)"))
  (if (`ActorComponent.ComponentHasTag` OtherComp "K")
    (`self.Success`)))

(event `EnhancedInput|/Game/ThirdPerson/Input/Actions/IA_Move`
  (params (ActionValue :type "Vector2D Structure") (ElapsedSeconds :type "Float (double-precision)") (TriggeredSeconds :type "Float (double-precision)") (InputAction :type "InputAction Object Reference" :default "/Game/ThirdPerson/Input/Actions/IA_Move.IA_Move"))
  (bind (_returnvalue_x _returnvalue_y) (`KismetMathLibrary.BreakVector2D` (`KismetMathLibrary.Normal2D` ActionValue)))
  (bind _platforma (`self.Platforma`))
  (bind (_relativerotation_roll _relativerotation_pitch) (`KismetMathLibrary.BreakRotator` (`SceneComponent.RelativeRotation` _platforma)))
  (:`Triggered`
    (`SceneComponent.K2_AddRelativeRotation` (`self.Platforma`) (`KismetMathLibrary.MakeRotator` (* _returnvalue_x (`self.Sensivity`)) (* _returnvalue_y (`self.Sensivity`))) false false)
    (`SceneComponent.K2_SetRelativeRotation` _platforma (`KismetMathLibrary.MakeRotator` (`KismetMathLibrary.FClamp` _relativerotation_roll -20.0 20.0) (`KismetMathLibrary.FClamp` _relativerotation_pitch -20.0 20.0)) false false)))

(event `self.Box1.OnComponentBeginOverlap`
  (params (OverlappedComponent :type "PrimitiveComponent Object Reference") (OtherActor :type "Actor Object Reference") (OtherComp :type "PrimitiveComponent Object Reference") (OtherBodyIndex :type Integer) (bFromSweep :type Boolean) (SweepResult :type "HitResult Structure (by ref)"))
  (if (== OtherComp (`self.Kula`))
    (`self.Fail`)))

(fn `UserConstructionScript`
  (`parent.UserConstructionScript`))