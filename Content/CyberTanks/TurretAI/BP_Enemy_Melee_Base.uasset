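; Base melee enemy for CyberTanks that spawns an attached saw actor and destroys it on its own destruction.
; Pawn sensing writes any spotted player vehicle to the AI blackboard.
; Attack sphere-traces WorldStatic objects ahead and switches to charge speed on hitting a player-tagged actor.
; Damage drains HP and energy: depleted energy briefly disables movement, depleted HP destroys the enemy.
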(event `OnDestroyed_Event` :!signature `self.OnDestroyed`
  (params (DestroyedActor :type "Actor Object Reference"))
  ; Spawn
  (`self.K2_DestroyActor` (stale `self.ReceiveBeginPlay` _returnvalue)))

(event `self.ReceiveBeginPlay`
  ; Spawn
  (bind _returnvalue (`|SpawnActorFromClass` "/Game/CyberTanks/TurretAI/BP_Saw_Base.BP_Saw_Base_C" (`SceneComponent.K2_GetComponentToWorld` (`self.RootComponent`)) "Undefined" "MultiplyWithRoot" null null))
  (add `self.OnDestroyed` (delegate `OnDestroyed_Event`))
  (`self.K2_AttachToComponent` _returnvalue (`self.RootComponent`) "None" "KeepWorld" "KeepWorld" "KeepRelative" true))

(event `Attack`
  (bind _returnvalue (`self.K2_GetActorLocation`))
  (bind _outhit (`KismetSystemLibrary.SphereTraceSingleForObjects` :`Start` _returnvalue :`End` (+ _returnvalue (* (`KismetMathLibrary.GetForwardVector` (`self.K2_GetActorRotation`)) 500.0)) :`Radius` 1500.0 :`ObjectTypes` (`|MakeArray` "ObjectTypeQuery1" :!type "EObjectTypeQuery Enum") :`DrawDebugType` "ForDuration"))
  (if (`self.ActorHasTag` (`.HitActor` (`GameplayStatics.BreakHitResult` _outhit)) "PlayerVehicle")
    (set `CharacterMovementComponent.MaxWalkSpeed` (`self.EnemyChargeSpeed`) (`self.CharacterMovement`))))

(event `self.PawnSensing.OnSeePawn`
  (params (Pawn :type "Pawn Object Reference"))
  (bind _returnvalue (`AIBlueprintHelperLibrary.GetBlackboard` (`AIBlueprintHelperLibrary.GetAIController` self)))
  ;[0.2109 0.8646 0.07655 0.5] OnSeePawn
  (`KismetSystemLibrary.PrintString` "WIDZE WIDZE WIDZE WIDZE WIDZE")
  (if (`self.ActorHasTag` Pawn "PlayerVehicle")
    (`BlackboardComponent.SetValueAsObject` _returnvalue "PlayerVehicle" Pawn)
    (`BlackboardComponent.SetValueAsBool` _returnvalue "playerSpotted?" true)
    (`KismetSystemLibrary.PrintString` (`KismetStringLibrary.Conv_BoolToString` (`BlackboardComponent.GetValueAsBool` _returnvalue "playerSpotted?")))))

(event `/Game/CyberTanks/EnergonComponent/BPI_Energon.Damage`
  (params (HPDamage :type "Float (double-precision)") (EnergyDamage :type "Float (double-precision)"))
  (bind _charactermovement (`self.CharacterMovement`))
  (set `self.HP` (- (`self.HP`) HPDamage))
  (set `self.Energy` (- (`self.Energy`) EnergyDamage))
  (`|ExecutionSequence`
    (:`then_0`
      (if (<= (`self.Energy`) 0.0)
        (`CharacterMovementComponent.SetMovementMode` _charactermovement "MOVE_None" 0)
        (`KismetSystemLibrary.Delay` 4.0)
        (`CharacterMovementComponent.SetMovementMode` _charactermovement "MOVE_Walking" 0)))
    (:`then_1`
      (if (<= (`self.HP`) 0.0)
        (`KismetSystemLibrary.PrintString` "Kill Logic")
        (`self.K2_DestroyActor`)))))

(fn `UserConstructionScript`)