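; Base offensive turret that spots player-tagged pawns with PawnSensing and fires physics-driven bullets at them.
; Each sighting stores the target location, yaws the base and barrel toward it, enters ATTACKING and restarts a one-second timer back to IDLE.
; While attacking, Tick triggers shots from the arrow toward that location, gated by a flag and delays that create bursts with longer pauses.
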(event `self.ReceiveTick`
  (params (DeltaSeconds :type "Float (single-precision)"))
  (switch `/Game/CyberTanks/TurretAI/EN_TurretState` (`self.TurretState`)
    (:`NewEnumerator1`
      (`self.TurretAttack`))))

(event `self.PawnSensing.OnSeePawn`
  (params (Pawn :type "Pawn Object Reference"))
  (bind _turretbase (`self.TurretBase`))
  (bind _gunbarrel (`self.GunBarrel`))
  (bind (_returnvalue_roll _returnvalue_pitch) (`KismetMathLibrary.BreakRotator` (`SceneComponent.K2_GetComponentRotation` _turretbase)))
  (bind (_returnvalue_roll_2 _returnvalue_pitch_2) (`KismetMathLibrary.BreakRotator` (`SceneComponent.K2_GetComponentRotation` _gunbarrel)))
  (bind (_returnvalue_roll_3 _returnvalue_pitch_3 _returnvalue_yaw) (`KismetMathLibrary.BreakRotator` (`KismetMathLibrary.FindLookAtRotation` (`self.K2_GetActorLocation`) (`self.Target Location`))))
  (`KismetSystemLibrary.PrintString` "Hello")
  (if (`self.ActorHasTag` Pawn "Player")
    (set `self.Target Location` (`self.K2_GetActorLocation` Pawn))
    (set `self.TurretState` "NewEnumerator1")
    (`SceneComponent.K2_SetRelativeRotation` _turretbase (`KismetMathLibrary.MakeRotator` _returnvalue_roll _returnvalue_pitch _returnvalue_yaw) false false)
    (`SceneComponent.K2_SetRelativeRotation` _gunbarrel (`KismetMathLibrary.MakeRotator` _returnvalue_roll_2 _returnvalue_pitch_2 _returnvalue_yaw) false false)
    (`KismetSystemLibrary.K2_ClearAndInvalidateTimerHandle` (`self.ResetTurretStateTimer`))
    (bind _returnvalue (`KismetSystemLibrary.K2_SetTimerDelegate` (delegate `ResetTurretState`) 1.0))
    (set `self.ResetTurretStateTimer` _returnvalue)))

(event `ResetTurretState`
  (set `self.TurretState` "NewEnumerator0"))

(event `TurretAttack`
  (bind _returnvalue (`SceneComponent.K2_GetComponentLocation` (`self.Arrow`)))
  (bind _returnvalue_2 (`KismetMathLibrary.GetDirectionUnitVector` _returnvalue (`self.Target Location`)))
  (if (not (`self.IsAttacking?`))
    (set `self.IsAttacking?` true)
    (bind _returnvalue_3 (`|SpawnActorFromClass` "/Game/CyberTanks/TankBase/Modules/CannonModule/BP_Bullet.BP_Bullet_C" (`KismetMathLibrary.MakeTransform` (+ _returnvalue (* _returnvalue_2 60.0))) "Undefined" "MultiplyWithRoot" null null))
    (`PrimitiveComponent.SetPhysicsLinearVelocity` (`/Game/CyberTanks/TankBase/Modules/CannonModule/BP_Bullet.BulletMesh` _returnvalue_3) (* _returnvalue_2 3000.0) false "None")
    (`KismetSystemLibrary.Delay` (`self.DelayBetweenAttacks`))
    (bind _result (`/Engine/EditorBlueprintResources/StandardMacros.IncrementInt` (`self.NumbersOfAttacksDone`))
      (:`  `
        (if (>= _result (`self.AttackFrequency`))
          (set `self.NumbersOfAttacksDone` 0)
          (`KismetSystemLibrary.Delay` (`self.DelayBetweenMultipleAttacks`)))
        (set `self.IsAttacking?` false)))))

(fn `UserConstructionScript`)