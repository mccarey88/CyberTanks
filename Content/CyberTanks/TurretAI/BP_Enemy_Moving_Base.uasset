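; Base moving enemy character that carries a shooting pawn, spawned above it and attached on BeginPlay, then destroyed along with it.
; A Damage event lowers HP and Energy: depleted energy disables movement for four seconds before restoring walking, and depleted HP destroys the actor.
; PawnSensing records the last seen time and writes pawns tagged PlayerVehicle and a spotted flag to the AI controller's blackboard.
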(event `OnDestroyed_Event` :!signature `self.OnDestroyed`
  (params (DestroyedActor :type "Actor Object Reference"))
  ; Spawn
  (`self.K2_DestroyActor` (stale `self.ReceiveBeginPlay` _returnvalue_2)))

(event `/Game/CyberTanks/EnergonComponent/BPI_Energon.Damage`
  (params (HPDamage :type "Float (double-precision)") (EnergyDamage :type "Float (double-precision)"))
  (bind _charactermovement (`self.CharacterMovement`))
  (set `self.HP` (- (`self.HP`) HPDamage))
  (set `self.Energy` (- (`self.Energy`) EnergyDamage))
  (`|ExecutionSequence`
    (:`then_0`
      (if (<= (`self.Energy`) 0.0)
        (`CharacterMovementComponent.SetMovementMode` _charactermovement "MOVE_None" 0)
        (`KismetSystemLibrary.Delay` 4.0)
        (`CharacterMovementComponent.SetMovementMode` _charactermovement "MOVE_Walking" 0)))
    (:`then_1`
      (if (<= (`self.HP`) 0.0)
        (`KismetSystemLibrary.PrintString` "Kill Logic")
        (`self.K2_DestroyActor`)))))

(event `self.ReceiveBeginPlay`
  (bind _returnvalue (`SceneComponent.K2_GetComponentToWorld` (`self.RootComponent`)))
  ; Spawn
  (bind _returnvalue_2 (`|SpawnActorFromClass` "/Game/CyberTanks/TurretAI/BP_ShootingPawn_Base.BP_ShootingPawn_Base_C" (`KismetMathLibrary.MakeTransform` (`KismetMathLibrary.MakeVector` (.x (.location _returnvalue)) (.y (.location _returnvalue)) (+ (.z (.location _returnvalue)) 50.0)) (.rotation _returnvalue) (.scale _returnvalue)) "Undefined" "MultiplyWithRoot" null null))
  (add `self.OnDestroyed` (delegate `OnDestroyed_Event`))
  (`self.K2_AttachToComponent` _returnvalue_2 (`self.RootComponent`) "None" "KeepWorld" "KeepWorld" "KeepRelative" true))

(event `self.PawnSensing.OnSeePawn`
  (params (Pawn :type "Pawn Object Reference"))
  (bind _returnvalue (`AIBlueprintHelperLibrary.GetBlackboard` (`AIBlueprintHelperLibrary.GetAIController` self)))
  ;[0.1388 1 0 0.5] OnSeePawn
  (set `self.LastSeenTime` (`GameplayStatics.GetTimeSeconds`))
  (if (`self.ActorHasTag` Pawn "PlayerVehicle")
    (`BlackboardComponent.SetValueAsObject` _returnvalue "PlayerVehicle" Pawn)
    (`BlackboardComponent.SetValueAsBool` _returnvalue "playerSpotted?" true)))

(fn `UserConstructionScript`)