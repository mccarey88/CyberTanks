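; BP_TestDPS is a test-map target actor for measuring damage, showing its health and energy on an attached widget.
; The Damage event applies HP and energy damage to its ACEnergon component, then refreshes the WBP_TestDPS display, as BeginPlay also does.
; The display receives current and maximum values plus the damage amounts from that single Damage call, with no accumulation or per-second calculation in this Blueprint.
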(event `self.ReceiveBeginPlay`
  (bind _ac_energon (`self.AC_Energon`))
  (bind _aswbp_test_dps (cast `/Game/CyberTanks/TestMap/Tester/WBP_TestDPS` (`WidgetComponent.GetWidget` (`self.Widget`)) :!label _label))
  (`/Game/CyberTanks/TestMap/Tester/WBP_TestDPS.Update Text` _aswbp_test_dps (`/Game/CyberTanks/EnergonComponent/AC_Energon.HP` _ac_energon) (`/Game/CyberTanks/EnergonComponent/AC_Energon.MaxHp` _ac_energon) (`/Game/CyberTanks/EnergonComponent/AC_Energon.Energy` _ac_energon) (`/Game/CyberTanks/EnergonComponent/AC_Energon.MaxEnergy` _ac_energon) (stale `/Game/CyberTanks/EnergonComponent/BPI_Energon.Damage` HPDamage) (stale `/Game/CyberTanks/EnergonComponent/BPI_Energon.Damage` EnergyDamage)))

(event `/Game/CyberTanks/EnergonComponent/BPI_Energon.Damage`
  (params (HPDamage :type "Float (double-precision)") (EnergyDamage :type "Float (double-precision)"))
  (`/Game/CyberTanks/EnergonComponent/AC_Energon.Damage` (`self.AC_Energon`) HPDamage EnergyDamage)
  (goto _label))

(fn `UserConstructionScript`)