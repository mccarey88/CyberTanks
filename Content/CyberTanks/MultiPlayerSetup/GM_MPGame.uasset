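; GM_MPGame is the CyberTanks game mode that sets up local multiplayer on BeginPlay.
; It creates additional local players with their own controllers, switches the default pawn to BP_ThirdPersonCharacter and restarts the first player.
; It then gives each PC_MPGame controller a minigame render target and material, matched by array index.
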(event `self.ReceiveBeginPlay`
  (for _ (range 4)
    (bind _returnvalue (`GameplayStatics.CreatePlayer` -1))
    (cast `/Game/CyberTanks/MultiPlayerSetup/PC_MPGame` _returnvalue))
  (set `self.DefaultPawnClass` "/Game/ThirdPerson/Blueprints/BP_ThirdPersonCharacter.BP_ThirdPersonCharacter_C")
  (`self.RestartPlayer` (`GameplayStatics.GetPlayerController` 0))
  ; Assigning render targets for minigames to each controller
  (bind _outactors (`GameplayStatics.GetAllActorsOfClass` "/Game/CyberTanks/MultiPlayerSetup/PC_MPGame.PC_MPGame_C"))
  (for (_array_element _array_index) _outactors
    (set `/Game/CyberTanks/MultiPlayerSetup/PC_MPGame.RenderTarget` (`|GetArrayItem` (`self.RenderTexturesForMiniGames`) _array_index) _array_element)
    (set `/Game/CyberTanks/MultiPlayerSetup/PC_MPGame.RenderMaterial` (`|GetArrayItem` (`self.MaterialForRT`) _array_index) _array_element)))

(fn `UserConstructionScript`)