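; Game instance for CyberTanks that persists the tank loadout (module names and vehicle base) in a single "test" save slot.
; On Init it async-loads and caches the BP_SaveGame, or, if none exists, writes a default loadout and quits so the game can be reopened.
; SaveGame copies the loadout from the first BP_Vehicle found into a fresh save object, overwriting the slot.
; Older save and debug-print chains remain unconnected.
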(event `self.ReceiveInit`
  ;[0 1 0.1 0.5] START
  (bind _returnvalue (`GameplayStatics.DoesSaveGameExist` "test"))
  (if _returnvalue
    (bind _savegame (`AsyncActionHandleSaveGame.AsyncLoadGameFromSlot` "test")
      (:`Completed`
        (set `self.SaveLoaded` true)
        (bind _asbp_save_game (cast `/Game/CyberTanks/MultiPlayerSetup/BP_SaveGame` _savegame))
        (set `self.Save Game` _asbp_save_game)))
    (else
      (`KismetSystemLibrary.PrintString` "didnt load game \nCreating save. \nGame will close. \nopen again" true true (struct :`R` 1.0 :`B` 0.026213 :`A` 1.0) 15.0)
      (`KismetSystemLibrary.DelayUntilNextTick`)
      (`KismetSystemLibrary.DelayUntilNextTick`)
      (`KismetSystemLibrary.DelayUntilNextTick`)
      (`self.CreateDefaultSave`)
      (`KismetSystemLibrary.Delay` 4.0)
      (`KismetSystemLibrary.QuitGame` null "Quit"))))

(event `SaveGame`
  (`KismetSystemLibrary.PrintString` "GameSaved" true true (struct :`R` 0.311259 :`G` 0.011792 :`B` 1.0 :`A` 1.0) 100.0)
  (bind _returnvalue (`GameplayStatics.GetActorOfClass` "/Game/CyberTanks/TankBase/Vehicle/BP_Vehicle.BP_Vehicle_C"))
  (bind _returnvalue_2 (`GameplayStatics.CreateSaveGameObject` "/Game/CyberTanks/MultiPlayerSetup/BP_SaveGame.BP_SaveGame_C"))
  (set `/Game/CyberTanks/MultiPlayerSetup/BP_SaveGame.ModuleNames` (`/Game/CyberTanks/TankBase/Vehicle/BP_Vehicle.ModuleNames` _returnvalue) _returnvalue_2)
  (set `/Game/CyberTanks/MultiPlayerSetup/BP_SaveGame.VehicleBaseName` (`/Game/CyberTanks/TankBase/Vehicle/BP_Vehicle.VehicleBaseName` _returnvalue) _returnvalue_2)
  (`GameplayStatics.SaveGameToSlot` _returnvalue_2 "test"))

(event `CreateDefaultSave`
  ; Default Save
  (bind _returnvalue (`GameplayStatics.CreateSaveGameObject` "/Game/CyberTanks/MultiPlayerSetup/BP_SaveGame.BP_SaveGame_C"))
  (set `/Game/CyberTanks/MultiPlayerSetup/BP_SaveGame.ModuleNames` (`|MakeArray` "NewEnumerator0" "NewEnumerator1" "NewEnumerator1" "NewEnumerator2" "NewEnumerator0" :!type "/Game/CyberTanks/TankConfiguration/ENUM_ModuleNames Enum") _returnvalue)
  (set `/Game/CyberTanks/MultiPlayerSetup/BP_SaveGame.VehicleBaseName` "NewEnumerator1" _returnvalue)
  (`GameplayStatics.SaveGameToSlot` _returnvalue "test"))