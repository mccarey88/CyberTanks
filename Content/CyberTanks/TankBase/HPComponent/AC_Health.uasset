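; Health component for CyberTanks tanks that tracks HP and a state of Invulnerable, FullyOperational, Damaged or Disabled.
; BeginPlay creates a paused invulnerability timer and calls FullRestore; FullRestore_Event refills HP, sets Invulnerable and unpauses the timer.
; Damage always subtracts HP, then CheckHPFunc derives the state unless Invulnerable, and Disabled fires HPZero.
; VulnerableAgain ends invulnerability and rechecks HP, so damage taken meanwhile still counts.
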(event `self.ReceiveBeginPlay`
  (bind _returnvalue (`KismetSystemLibrary.K2_SetTimerDelegate` (`|CreateDelegate` :!event `VulnerableAgain`) (`self.InvulnerableTime`)))
  (bind _output_get (set `self.InvulnerableHandler` _returnvalue))
  (`KismetSystemLibrary.K2_PauseTimerHandle` _output_get)
  (`self.FullRestore`))

(event `Damage`
  (params (Ammount :type "Float (double-precision)"))
  (set `self.HP` (- (`self.HP`) Ammount))
  (`self.CheckHP`))

(event `CheckHP`
  (bind _newparam (`self.CheckHPFunc`))
  (switch `/Game/CyberTanks/TankBase/HPComponent/ENUM_HPState` _newparam
    (:`NewEnumerator2`
      (`self.HPZero`))))

(event `FullRestore_Event`
  (set `self.HP` (`self.MaxHp`))
  (`self.InvulnerableState`))

(event `InvulnerableState`
  (set `self.HPState` "NewEnumerator4")
  (`KismetSystemLibrary.K2_UnPauseTimerHandle` (`self.InvulnerableHandler`)))

(event `VulnerableAgain`
  (set `self.HPState` "NewEnumerator0")
  (`self.CheckHP`))

(fn `CheckHPFunc`
  (returns (NewParam :type "/Game/CyberTanks/TankBase/HPComponent/ENUM_HPState Enum"))
  (if (`|EnumEquality` (`self.HPState`) "NewEnumerator4")
    (return "NewEnumerator4")
    (elif (<= (`self.HP`) 0.0)
      (bind _output_get (set `self.HPState` "NewEnumerator2"))
      (return _output_get)
      (elif (< (`self.HP`) (`self.MaxHp`))
        (bind _output_get_2 (set `self.HPState` "NewEnumerator1"))
        (return _output_get_2)
        (elif (== (`self.HP`) (`self.MaxHp`))
          (bind _output_get_3 (set `self.HPState` "NewEnumerator0"))
          (return _output_get_3))))))