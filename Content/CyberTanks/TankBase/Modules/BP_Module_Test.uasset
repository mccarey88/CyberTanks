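; BP_Module_Test is a test tank module for CyberTanks that exercises the health component and input handling of its parent module class.
; On BeginPlay it runs the parent logic, then damages its ACHealth component and immediately fully restores it.
; Move input prints the module's name and value as debug text, while Interact starts the mini-game event.
; An interact debug print remains unconnected, and the construction script only calls the parent.
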(event `self.ReceiveBeginPlay`
  (bind _ac_health (`self.AC_Health`))
  (`parent.ReceiveBeginPlay`)
  (`/Game/CyberTanks/TankBase/HPComponent/AC_Health.Damage` _ac_health 100.0)
  (`/Game/CyberTanks/TankBase/HPComponent/AC_Health.FullRestore` _ac_health))

(event `EnhancedInput|/Game/ThirdPerson/Input/Actions/IA_Move`
  (params (ActionValue :type "Vector2D Structure") (ElapsedSeconds :type "Float (double-precision)") (TriggeredSeconds :type "Float (double-precision)") (InputAction :type "InputAction Object Reference" :default "/Game/ThirdPerson/Input/Actions/IA_Move.IA_Move"))
  (:`Triggered`
    (`KismetSystemLibrary.PrintText` (`|FormatText` "name:{a} \nvalue:{b}" self (`KismetStringLibrary.Conv_Vector2dToString` ActionValue)))))

(event `EnhancedInput|/Game/ThirdPerson/Input/Actions/IA_Interact`
  (params (ActionValue :type Boolean) (ElapsedSeconds :type "Float (double-precision)") (TriggeredSeconds :type "Float (double-precision)") (InputAction :type "InputAction Object Reference" :default "/Game/ThirdPerson/Input/Actions/IA_Interact.IA_Interact"))
  (:`Started`
    (`self.StartMiniGameEvent`)))

(fn `UserConstructionScript`
  (`parent.UserConstructionScript`))