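; BP_Bullet is the projectile actor for the tank cannon module, carrying a ProjectileMovement component and dealing damage on impact.
; Its Hit event prints the hit actor, distance and location for debugging, then checks the actor's class for BPI_Energon.
; When the interface is present, OnPlayerHit sends a fixed HP-only DamageMessage to that actor and the bullet is destroyed.
; Other hits leave the bullet alive, and the bounce handler is empty.
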(event `self.ProjectileMovement.OnProjectileBounce`
  (params (ImpactResult :type "HitResult Structure (by ref)") (ImpactVelocity :type "Vector Structure (by ref)")))

(event `self.ReceiveHit`
  (params (MyComp :type "PrimitiveComponent Object Reference") (Other :type "Actor Object Reference") (OtherComp :type "PrimitiveComponent Object Reference") (bSelfMoved :type Boolean) (HitLocation :type "Vector Structure") (HitNormal :type "Vector Structure") (NormalImpulse :type "Vector Structure") (Hit :type "HitResult Structure (by ref)"))
  (bind (_bblockinghit _binitialoverlap _time _distance _location _impactpoint _normal _impactnormal _physmat _hitactor) (`GameplayStatics.BreakHitResult` Hit))
  (`KismetSystemLibrary.PrintText` (`|FormatText` "HIT, \n-actor:{a} \n-distance:{b} \n-location:{c}" _hitactor _distance (`|FormatText` "{a},{b},{c}" (.x _location) (.y _location) (.z _location))))
  (if (`KismetSystemLibrary.DoesClassImplementInterface` (`GameplayStatics.GetObjectClass` _hitactor) "/Game/CyberTanks/EnergonComponent/BPI_Energon.BPI_Energon_C")
    (`self.OnPlayerHit`)
    (`self.K2_DestroyActor`)))

(event `OnPlayerHit`
  ; Event
  (message `/Game/CyberTanks/EnergonComponent/BPI_Energon.Damage` (`.HitActor` (`GameplayStatics.BreakHitResult` (stale `self.ReceiveHit` Hit))) 10.0 0.0))

(fn `UserConstructionScript`)