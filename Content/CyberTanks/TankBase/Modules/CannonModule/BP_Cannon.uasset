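; BP_Cannon is the tank's cannon module, which aims and fires bullets.
; Aim rotates the Sphere component by the input's X as yaw and Y as pitch, then clamps both axes to a symmetric limit and zeroes roll.
; Shoot spawns a BP_Bullet at the BulletSpawnPoint transform and prints a debug "Bang" message.
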(event `Aim`
  (params (InputValue :type "Vector2D Structure"))
  (bind (_x _y) (`KismetMathLibrary.BreakVector2D` InputValue))
  (bind _sphere (`self.Sphere`))
  (bind (_relativerotation_roll _relativerotation_pitch _relativerotation_yaw) (`KismetMathLibrary.BreakRotator` (`SceneComponent.RelativeRotation` _sphere)))
  (`SceneComponent.K2_AddRelativeRotation` (`self.Sphere`) (`KismetMathLibrary.MakeRotator` 0.0 0.0 _x) false false)
  (`SceneComponent.K2_AddRelativeRotation` (`self.Sphere`) (`KismetMathLibrary.MakeRotator` 0.0 _y) false false)
  (`SceneComponent.K2_SetRelativeRotation` _sphere (`KismetMathLibrary.MakeRotator` 0.0 (`KismetMathLibrary.FClamp` _relativerotation_pitch -45.0 45.0) (`KismetMathLibrary.FClamp` _relativerotation_yaw -45.0 45.0)) false false))

(event `Shoot`
  (`|SpawnActorFromClass` "/Game/CyberTanks/TankBase/Modules/CannonModule/BP_Bullet.BP_Bullet_C" (`SceneComponent.K2_GetComponentToWorld` (`self.BulletSpawnPoint`)) "Undefined" "MultiplyWithRoot" null null)
  (`KismetSystemLibrary.PrintString` "Bang"))

(fn `UserConstructionScript`)