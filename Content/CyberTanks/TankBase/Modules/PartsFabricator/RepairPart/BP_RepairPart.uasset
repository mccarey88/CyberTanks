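; BP_RepairPart is a physics-simulated repair part for the tank's parts fabricator module.
; On BeginPlay it looks up its Name in DT_RepairParts, applies that row's mesh and enables physics.
; It then sets RepairNeed by matching the row's name against the ENUM_RepairNeed entries converted to names.
; WhatRepairPart reports that repair need along with whether the part is carried.
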(event `self.ReceiveBeginPlay`
  (bind _returnvalue (`|GetDataTableRow` "/Game/CyberTanks/TankBase/Modules/PartsFabricator/RepairPart/DT_RepairParts.DT_RepairParts" (`self.Name`))
    (:`then`
      (bind (_name _mesh) (break `/Game/CyberTanks/TankBase/Modules/PartsFabricator/RepairPart/STRUCT_RepairPart` _returnvalue))
      (`StaticMeshComponent.SetStaticMesh` (`self.StaticMesh`) _mesh)
      (`PrimitiveComponent.SetSimulatePhysics` (`self.StaticMesh`) true)
      (bind _enumvalue (foreach `/Game/CyberTanks/TankBase/Modules/PartsFabricator/ENUM_RepairNeed` false)
        (:`LoopBody`
          (if (== (`KismetStringLibrary.Conv_StringToName` (`|GetEnumeratorNameAsString` _enumvalue)) _name)
            (set `self.RepairNeed` _enumvalue)))
        (:`then`)))))

(fn `UserConstructionScript`)

(fn `WhatRepairPart`
  (returns (RepairNeedPart :type "/Game/CyberTanks/TankBase/Modules/PartsFabricator/ENUM_RepairNeed Enum") (`PartCarried?` :type Boolean))
  (return (`self.RepairNeed`) (`self.Carried?`)))